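; Obstacle actor that drifts through the world along a movement direction while spinning.
; The construction script randomizes its rotation rate on a RotatingMovement component, a uniform scale and a speed, each of the latter two within a min/max range.
; Tick offsets the actor by direction, speed and delta time without sweeping, so movement does not stop on collisions.
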(event `self.ReceiveTick`
  (params (DeltaSeconds :type "Float (single-precision)"))
  (`self.K2_AddActorWorldOffset` (* (`self.Movement Direction`) (* DeltaSeconds (`self.Current Speed`)))))

(fn `UserConstructionScript`
  (set `RotatingMovementComponent.RotationRate` (`KismetMathLibrary.RandomRotator` false) (`self.RotatingMovement`))
  (`self.SetActorScale3D` (`KismetMathLibrary.Conv_DoubleToVector` (`KismetMathLibrary.RandomFloatInRange` (`self.Random Scale Min`) (`self.Random Scale Max`))))
  (set `self.Current Speed` (`KismetMathLibrary.RandomFloatInRange` (`self.Speed Min`) (`self.Speed Max`))))