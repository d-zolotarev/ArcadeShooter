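; Player spaceship that moves sideways, fires plasma bolts and creates its HUD widget on begin play.
; Space or left click spawns a bolt with a sound while the ship is alive.
; A first hit turns on damage particles, which healing clears; a hit while damaged explodes and hides the ship, then sets a timer to restart the game.
; It also keeps a score counter, incremented through an event.
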(event `self.ReceiveBeginPlay`
  (bind _returnvalue (`|CreateWidget` "/Game/StartGameMenu/Hero_HUD_Widget.Hero_HUD_Widget_C" (`GameplayStatics.GetPlayerController` 0)))
  (`UserWidget.AddToViewport` _returnvalue 0))

(event `InputAxis|MoveRight`
  (params (AxisValue :type "Float (single-precision)"))
  (`self.AddMovementInput` (`self.GetActorRightVector`) AxisValue))

(event `Key|SpaceBar`
  (params (Key :type "Key Structure"))
  (bind _returnvalue (`self.K2_GetActorLocation`))
  (:`Pressed`
    (if (not (`self.IsDead`)) :!label _label
      (`GameplayStatics.PlaySoundAtLocation` "/Game/Audio/zapulnuvshiy-lazernyiy-stvol.zapulnuvshiy-lazernyiy-stvol" _returnvalue (struct) 1.0 1.0 0.0 null null null)
      (`|SpawnActorFromClass` "/Game/Blueprints/Plasma_Bolt.Plasma_Bolt_C" (`KismetMathLibrary.Conv_VectorToTransform` _returnvalue) "Undefined" "OverrideRootScale" null null))))

(event `Key|LeftMouseButton`
  (params (Key :type "Key Structure"))
  (:`Pressed`
    (goto _label)))

(event `UpdateScore`
  (bind _result (`/Engine/EditorBlueprintResources/StandardMacros.IncrementInt` (`self.Score`))
    (:`  `
      (if (== _result 65535)
        (set `self.Score` 0)))))

(fn `Heal Damage`
  (set `self.Is Damaged` false)
  (`ActorComponent.Deactivate` (`self.Damage Partical System`)))

(fn `On Death`
  (bind _returnvalue (`self.K2_GetActorLocation`))
  (`GameplayStatics.SpawnEmitterAtLocation` "/Game/StarterContent/Particles/P_Explosion.P_Explosion" _returnvalue)
  (`GameplayStatics.PlaySoundAtLocation` "/Game/Audio/kosmicheskiy-vzryiv-32082.kosmicheskiy-vzryiv-32082" _returnvalue (struct) 1.0 1.0 0.0 null null null)
  (set `self.IsDead` true)
  (`self.SetActorHiddenInGame` true)
  (`self.SetActorEnableCollision` false)
  (`KismetSystemLibrary.K2_SetTimer` (`GameplayStatics.GetGameMode`) "RestartGame" 3.0))

(fn `Take Damage`
  (if (`self.Is Damaged`)
    (`self.On Death`)
    (else
      (set `self.Is Damaged` true)
      (`GameplayStatics.PlaySoundAtLocation` "/Game/Audio/kosmicheskiy-vzryiv-32082.kosmicheskiy-vzryiv-32082" (`self.K2_GetActorLocation`) (struct) 1.0 1.0 0.0 null null null)
      (`ActorComponent.Activate` (`self.Damage Partical System`) false))))

(fn `UserConstructionScript`)