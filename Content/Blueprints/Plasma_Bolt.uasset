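; Plasma bolt actor that destroys asteroids it overlaps and credits the player's score.
; On overlap with an Asteroid, it spawns an explosion emitter and sound at its own location, then calls UpdateScore on the player's Hero_Spaceship pawn.
; Both bolt and asteroid are destroyed only after that pawn cast succeeds; the graph contains no movement logic.
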(event `self.ReceiveActorBeginOverlap`
  (params (OtherActor :type "Actor Object Reference"))
  (bind _returnvalue (`self.K2_GetActorLocation`))
  (bind _asasteroid (cast `/Game/Blueprints/Asteroid` OtherActor))
  (`GameplayStatics.SpawnEmitterAtLocation` "/Game/StarterContent/Particles/P_Explosion.P_Explosion" _returnvalue)
  (`GameplayStatics.PlaySoundAtLocation` "/Game/StarterContent/Audio/Explosion01.Explosion01" _returnvalue (struct) 1.0 1.0 0.0 null null null)
  (bind _ashero_spaceship (cast `/Game/Blueprints/Hero_Spaceship` (`GameplayStatics.GetPlayerPawn` 0)))
  (`/Game/Blueprints/Hero_Spaceship.UpdateScore` _ashero_spaceship)
  (`self.K2_DestroyActor`)
  (`self.K2_DestroyActor` _asasteroid))

(fn `UserConstructionScript`
  (`parent.UserConstructionScript`))